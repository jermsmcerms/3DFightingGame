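; Player character Blueprint that takes clockwise and counter-clockwise axis input for movement based on a Spline reference.
; Both axes run identical logic, scaling controller yaw and movement input by the axis value from GetRotationAndLocationAlongSpline.
; That helper always samples the spline start (Lerp alpha fixed at zero) in local space, substituting actor Z.
; The returned location is passed as the movement direction, so nothing tracks progress along the spline.
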(event EventBeginPlay)

(event Input|AxisEvents|InputAxisMoveClockwise
  (params (AxisValue :type Float%20%28single-precision%29))
  (bind (_location _rotation) (CallFunction|GetRotationandLocationAlongSpline))
  (Pawn|Input|AddControllerYawInput (* (.yaw _rotation) AxisValue))
  (Pawn|Input|AddMovementInput _location AxisValue false))

(event Input|AxisEvents|InputAxisMoveCounterClockwise
  (params (AxisValue :type Float%20%28single-precision%29))
  (bind (_location _rotation) (CallFunction|GetRotationandLocationAlongSpline))
  (Pawn|Input|AddControllerYawInput (* (.yaw _rotation) AxisValue))
  (Pawn|Input|AddMovementInput _location AxisValue false))

(fn ConstructionScript)

(fn GetRotationandLocationAlongSpline
  (bind _spline (Variables|Default|GetSpline))
  (bind _returnvalue (Spline|GetSplineLength _spline))
  (bind _returnvalue_2 (Math|Float|Lerp 0.0 _returnvalue 0.0))
  (bind _returnvalue_3 (Spline|GetLocationatDistanceAlongSpline _spline _returnvalue_2 "Local"))
  (return (Math|Vector|MakeVector (.x _returnvalue_3) (.y _returnvalue_3) (.z (Transformation|GetActorLocation))) (Math|Rotator|MakeRotator 0.0 0.0 (.yaw (Spline|GetRotationatDistanceAlongSpline _spline (Math|Float|Lerp 0.0 (Spline|GetSplineLength _spline) 0.0) "Local")))))